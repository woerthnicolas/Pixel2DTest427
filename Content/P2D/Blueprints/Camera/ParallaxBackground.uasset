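; Parallax background actor for a 2D game that follows the camera horizontally and scrolls layered textures.
; The construction script builds each configured layer from textured planes alternating left and right, with dynamic materials and translucent sort priority.
; BeginPlay spawns a BP_CameraFollower at the player's camera.
; Tick matches its X and drives each layer's wrapped TextureOffset from follower velocity divided by layer ParallaxSpeed, so higher values scroll slower.
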(event EventBeginPlay
  (bind _returnvalue (Class|P2DGameMode|GetInstance))
  (bind _returnvalue_2 (Class|P2DGameMode|GetPlayerCharacter _returnvalue))
  (Utilities|IsValid _returnvalue_2
    (:Is%20Valid
      (bind _output_get (Variables|References|SetCharRef _returnvalue_2))
      (Variables|Default|SetCamera (Variables|/Script/Pixel2DTest427.P2DCharacter|GetCameraComp _output_get))
      (bind _returnvalue_3 (Game|SpawnActorfromClass "/Game/P2D/Blueprints/Camera/BP_CameraFollower.BP_CameraFollower_C" (Math|Transform|MakeTransform (Transformation|GetWorldLocation (Variables|Default|GetCamera)) "0, 0, 0" "1,1,1") "Undefined" 0 0))
      (Variables|References|SetCameraFollower _returnvalue_3)
      (for _array_element (Variables|Editable|GetParallaxLayers)
        (Utilities|Array|Add (Variables|NotEditable|GetparallaxOffset) 0.0)
        (Utilities|Array|Add (Variables|NotEditable|GetparallaxSpeed) 0.0)))
    (:Is%20Not%20Valid
      (Development|PrintString (Utilities|GetDisplayName _returnvalue_2)))))

(event Collision|EventActorBeginOverlap
  (params (OtherActor :type Actor%20Object%20Reference)))

(event EventTick
  (params (DeltaSeconds :type Float%20%28single-precision%29))
  (bind _returnvalue (Transformation|GetActorLocation))
  (bind _camerafollower (Variables|References|GetCameraFollower))
  (Variables|NotEditable|Settime DeltaSeconds)
  (Transformation|SetActorLocation (Math|Vector|MakeVector (.x (Transformation|GetActorLocation (Variables|References|GetCameraFollower))) (.y _returnvalue) (.z _returnvalue)) false false)
  (for (_array_element _array_index) (Variables|Editable|GetParallaxLayers)
    (Utilities|Array|SetArrayElem (Variables|NotEditable|GetparallaxSpeed) _array_index (/ (* (Variables|/Game/P2D/Blueprints/Camera/BP_CameraFollower.BP_CameraFollower_C|Getspeed _camerafollower) (.x (Variables|/Game/P2D/Blueprints/Camera/BP_CameraFollower.BP_CameraFollower_C|Getdirection _camerafollower))) (.ParallaxSpeed (Utilities|Struct|BreakParallaxLayer _array_element))) true)
    (Utilities|Array|SetArrayElem (Variables|NotEditable|GetparallaxOffset) _array_index (+ (Utilities|Array|Get(acopy) (Variables|NotEditable|GetparallaxOffset) _array_index) (* (Variables|NotEditable|Gettime) (Utilities|Array|Get(acopy) (Variables|NotEditable|GetparallaxSpeed) _array_index))) true)
    (if (> (Math|Float|Absolute(Float) (Utilities|Array|Get(acopy) (Variables|NotEditable|GetparallaxOffset) _array_index)) 1.0)
      (Utilities|Array|SetArrayElem (Variables|NotEditable|GetparallaxOffset) _array_index (.Remainder (Math|Float|Division(WholeandRemainder) (Utilities|Array|Get(acopy) (Variables|NotEditable|GetparallaxOffset) _array_index) 1.0)) true))
    (for _array_element_2 (.StaticMeshes (Utilities|Struct|BreakParallaxMeshes (Utilities|Array|Get(acopy) (Variables|NotEditable|GetParallaxMeshContainer) _array_index)))
      (Rendering|Material|SetScalarParameterValueonMaterials _array_element_2 "TextureOffset" (Utilities|Array|Get(acopy) (Variables|NotEditable|GetparallaxOffset) _array_index)))))

(fn ConstructionScript
  ;[1 1 1] Setup the Actor layers and parameters
  (for (_array_element _array_index) (Variables|Editable|GetParallaxLayers)
    (for _index (range 1 (.Amount (Utilities|Struct|BreakParallaxLayer _array_element)))
      (bind _returnvalue (AddComponent|AddStaticMeshComponent false (Math|Transform|MakeTransform (Math|Vector|MakeVector (+ (.X (Math|Vector|BreakVector (LocalVariables|GetLocation))) (.LayerXOffset (Utilities|Struct|BreakParallaxLayer _array_element))) (+ (.Y (Math|Vector|BreakVector (LocalVariables|GetLocation))) (.LayerYOffset (Utilities|Struct|BreakParallaxLayer _array_element))) (+ (.Z (Math|Vector|BreakVector (LocalVariables|GetLocation))) (.LayerZOffset (Utilities|Struct|BreakParallaxLayer _array_element)))) "0, 0, 0" (* (Math|Vector|MakeVector (.XScale (Utilities|Struct|BreakParallaxLayer _array_element)) 1.0 (.ZScale (Utilities|Struct|BreakParallaxLayer _array_element))) (.GlobalScale (Utilities|Struct|BreakParallaxLayer _array_element))))))
      (Rendering|SetTranslucentSortPriority _returnvalue (.LayerSortPriority (Utilities|Struct|BreakParallaxLayer _array_element)))
      (Utilities|Array|Add (LocalVariables|GettempMeshContainer) _returnvalue)
      (Components|StaticMesh|SetStaticMesh _returnvalue "/Game/Pixel2D/Meshes/BasicPlane.BasicPlane")
      (bind _returnvalue_2 (Rendering|Material|CreateDynamicMaterialInstance (Variables|Editable|GetParallaxMaterial) "None" "None" :!class /Script/Engine.KismetMaterialLibrary))
      (bind _output_get (Variables|References|SetParallaxMaterialInstance _returnvalue_2))
      (Rendering|Material|SetTextureParameterValue _output_get "Parallaxtexture" (.Texture (Utilities|Struct|BreakParallaxLayer _array_element)))
      (Rendering|Material|SetMaterial _returnvalue 0 (Variables|References|GetParallaxMaterialInstance))
      (Utilities|FlowControl|FlipFlop
        (:A
          (LocalVariables|SetLocation (Math|Vector|MakeVector (+ (* (* _index 1e+02) (* (.XScale (Utilities|Struct|BreakParallaxLayer _array_element)) (.GlobalScale (Utilities|Struct|BreakParallaxLayer _array_element)))) (.x (LocalVariables|GetLocation))) (.y (LocalVariables|GetLocation)) (.z (LocalVariables|GetLocation)))))
        (:B
          (LocalVariables|SetLocation (Math|Vector|MakeVector (+ (.x (LocalVariables|GetLocation)) (* (* _index -1e+02) (* (.XScale (Utilities|Struct|BreakParallaxLayer _array_element)) (.GlobalScale (Utilities|Struct|BreakParallaxLayer _array_element))))) (.y (LocalVariables|GetLocation)) (.z (LocalVariables|GetLocation)))))))
    (Utilities|Array|SetArrayElem (Variables|NotEditable|GetParallaxMeshContainer) _array_index (Utilities|Struct|MakeParallaxMeshes (LocalVariables|GettempMeshContainer) _array_index) true)
    (LocalVariables|SetLocation "0, 0, 0")
    (Utilities|Array|Clear (LocalVariables|GettempMeshContainer))))