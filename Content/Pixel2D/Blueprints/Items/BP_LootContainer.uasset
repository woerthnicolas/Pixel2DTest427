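; BP_LootContainer is a 2D loot chest that releases its stored items when interacted with.
; The first Interact plays a use sound, has LootDropComponent spawn all items and switches the Paper2D flipbook to a non-looping open animation.
; A WasOpened flag, reset on BeginPlay, limits this to one use, with later attempts only printing a message.
; The construction script assigns a new GUID as UniqueID whenever it runs.
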(event EventBeginPlay
  (Variables|Default|SetwasOpened? false))

(event Collision|EventActorBeginOverlap
  (params (OtherActor :type Actor%20Object%20Reference)))

(event EventTick
  (params (DeltaSeconds :type Float%20%28single-precision%29)))

(event EventInteract
  (params (Interactor :type Actor%20Object%20Reference))
  (bind _paperflipbook (Variables|Default|GetPaperFlipbook))
  ;[1 1 1] Spawns all stored items
  (if (Variables|Default|GetwasOpened?)
    (Development|PrintString (Utilities|String|Append (Utilities|GetDisplayName self) "" "was already opened!"))
    (else
      (Variables|Default|SetwasOpened? true)
      (Audio|PlaySoundatLocation (Variables|Default|GetOnUseSound) (Transformation|GetActorLocation) "0, 0, 0" 1.0 1.0 0.0 0 0 0)
      (Default|SpawnAllStoredItems (Variables|Default|GetLootDropComponent))
      (Sprite|SetFlipbook _paperflipbook "/Game/Pixel2D/FlipBooks/Final/FB_Chest_Open.FB_Chest_Open")
      (Components|Timeline|SetLooping _paperflipbook false))))

(fn ConstructionScript
  (Variables|Default|SetuniqueID (Guid|NewGuid)))